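; Third-person shooter character Blueprint that fires a test hitscan shot on left mouse click.
; The click routes through server-named events to an authority check, so only the authority runs the trace and damage.
; A long line trace runs from TraceStart along the follow camera's forward vector, with an optional debug draw.
; Hit TestCube_BP actors receive random damage at the impact point.
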(event `TraceDebug`
  (params (Start :type "Vector Structure") (End :type "Vector Structure"))
  (`KismetSystemLibrary.LineTraceSingleForObjects` :`Start` Start :`End` End :`ObjectTypes` (`|MakeArray` "ObjectTypeQuery1" "ObjectTypeQuery2" "ObjectTypeQuery3" "ObjectTypeQuery4" "ObjectTypeQuery5" "ObjectTypeQuery6" :!type "EObjectTypeQuery Enum") :`bTraceComplex` true :`DrawDebugType` "ForDuration"))

(event `Key|LeftMouseButton`
  (params (Key :type "Key Structure"))
  (:`Pressed`
    (`self.Serv_Test`)))

(event `Serv_Test`
  (`self.AuthoritiveServ_Test`))

(event `AuthoritiveServ_Test`
  (bind _returnvalue (`SceneComponent.K2_GetComponentLocation` (`self.TraceStart`)))
  (bind _returnvalue_2 (+ _returnvalue (* (`SceneComponent.GetForwardVector` (`self.FollowCamera`)) 10000.0)))
  (`/Engine/EditorBlueprintResources/ActorMacros.Switch Has Authority`
    (:`Authority`
      (if (`self.Debug`)
        (`self.TraceDebug` _returnvalue _returnvalue_2))
      (bind _outhit (`KismetSystemLibrary.LineTraceSingleForObjects` _returnvalue _returnvalue_2 (`|MakeArray` "ObjectTypeQuery1" "ObjectTypeQuery2" "ObjectTypeQuery3" "ObjectTypeQuery4" "ObjectTypeQuery5" "ObjectTypeQuery6" :!type "EObjectTypeQuery Enum") true))
      (bind (_bblockinghit _binitialoverlap _time _distance _location _impactpoint _normal _impactnormal _physmat _hitactor) (`GameplayStatics.BreakHitResult` _outhit))
      (bind _astest_cube_bp (cast `/Game/EntityBlueprints/TestCube_BP` _hitactor))
      (`/Game/EntityBlueprints/TestCube_BP.DoDamage` _astest_cube_bp (`KismetMathLibrary.RandomFloatInRange` 10.0 30.0) _impactpoint))))

(fn `UserConstructionScript`)