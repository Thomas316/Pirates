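; A networked test cube that players can interact with to toggle its color, and shoot to push and destroy.
; The authority handles toggling, damage, radial impulse and delayed destruction, with interactions forwarded through ServerInteract.
; RepNotifies on color and health update a dynamic material on clients.
; At zero health, the health RepNotify disables collision, hides the authoritative actor and spawns explosion FX on remotes before destruction.
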(event `self.ReceiveBeginPlay`
  (`|ExecutionSequence`
    (:`then_0`
      ;[1 1 1] Initialize the cube's CurrentHealth variable if we're on the authoritative worker.
      (if (`self.HasAuthority`)
        (set `self.CurrentHealth` (`self.MaxHealth`))))
    (:`then_1`
      ;[1 1 1] Make sure the object has a dynamic material if we're on the client, so we can change its color.
      (if (not (`KismetSystemLibrary.IsServer`))
        (`self.InitMaterial`)
        (`self.UpdateBaseColor`)
        (`self.UpdateColorFromHealth`)))))

(event `ServerInteract`
  ;[1 1 1] Respond to the Interact interface event by triggering a server interaction (if we're not on a server), or changing the IsColor1 variable (if we're authoritative).
  (if (`self.HasAuthority`) :!label _label
    (set `self.IsColor1` (not (`self.IsColor1`)))))

(event `Interact_1`
  ;[1 1 1] Respond to the Interact interface event by triggering a server interaction (if we're not on a server), or changing the IsColor1 variable (if we're authoritative).
  (if (`KismetSystemLibrary.IsServer`)
    (goto _label)
    (else
      (`self.ServerInteract`))))

(event `DoDamage`
  (params (Damage :type "Float (double-precision)") (`Hit Location` :type "Vector Structure"))
  ;[1 1 1] React to damage events from gunshots. Apply damage and destroy the cube if health hits 0.
  (if (`self.HasAuthority`)
    (`|ExecutionSequence`
      (:`then_0`
        (`self.ApplyDamage` (`KismetMathLibrary.FTrunc` Damage))
        (if (<= (`self.CurrentHealth`) 0)
          (`KismetSystemLibrary.Delay` 1.0) ; Delay destroying the actor so the VFX have time to show up in clients.
          (`self.K2_DestroyActor`)))
      (:`then_1`
        ;[1 1 1] React to point damage events by applying an impulse to the cube. note that this will execute *alongside* the AnyDamage event, so we will both add inpulse and decrement health.
        (`PrimitiveComponent.AddRadialImpulse` (`self.Box`) `Hit Location` 50.0 20000.0 "RIF_Constant" false)))))

(fn `ApplyDamage`
  (params (Amount :type Integer))
  (set `self.CurrentHealth` (- (`self.CurrentHealth`) (`KismetMathLibrary.Min` Amount (`self.CurrentHealth`)))))

(fn `InitMaterial`
  (if (not (`KismetSystemLibrary.IsValid` (`self.MaterialInstanceDynamic`)))
    (bind _returnvalue (`PrimitiveComponent.CreateDynamicMaterialInstance` (`self.Mesh`) 0 null "None"))
    (set `self.MaterialInstanceDynamic` _returnvalue)))

(fn `OnRep_CurrentHealth`
  (`|ExecutionSequence`
    (:`then_0`
      (if (not (`KismetSystemLibrary.IsServer`))
        (`self.UpdateColorFromHealth`)))
    (:`then_1`
      (if (<= (`self.CurrentHealth`) 0)
        (`PrimitiveComponent.SetCollisionEnabled` (`self.Box`) "NoCollision") ; bCollisionEnabled isn't replicated, so we need to disable it on all workers.
        (`/Engine/EditorBlueprintResources/ActorMacros.Switch Has Authority`
          (:`Authority`
            (`self.SetActorHiddenInGame` true))
          (:`Remote`
            (`self.SpawnExplosion`)))))))

(fn `OnRep_IsColor1`
  (if (not (`KismetSystemLibrary.IsServer`))
    (`self.UpdateBaseColor`)))

(fn `SpawnExplosion`
  (bind _explosionfx (`self.ExplosionFX`))
  (`/Engine/EditorBlueprintResources/StandardMacros.IsValid` _explosionfx
    (:`Is Valid`
      (`GameplayStatics.SpawnEmitterAtLocation` _explosionfx (`self.K2_GetActorLocation`)))))

(fn `UpdateBaseColor`
  (bind _materialinstancedynamic (`self.MaterialInstanceDynamic`))
  (`/Engine/EditorBlueprintResources/StandardMacros.IsValid` _materialinstancedynamic
    (:`Is Valid`
      (if (`self.IsColor1`)
        (`MaterialInstanceDynamic.SetVectorParameterValue` _materialinstancedynamic "BaseColor" (`self.Color1`))
        (else
          (`MaterialInstanceDynamic.SetVectorParameterValue` _materialinstancedynamic "BaseColor" (`self.Color2`)))))))

(fn `UpdateColorFromHealth`
  (bind _materialinstancedynamic (`self.MaterialInstanceDynamic`))
  (`/Engine/EditorBlueprintResources/StandardMacros.IsValid` _materialinstancedynamic
    (:`Is Valid`
      (`MaterialInstanceDynamic.SetScalarParameterValue` _materialinstancedynamic "CurrentHealth" (/ (`KismetMathLibrary.Conv_IntToDouble` (`self.CurrentHealth`)) (`KismetMathLibrary.Conv_IntToDouble` (`self.MaxHealth`)))))))

(fn `UserConstructionScript`)